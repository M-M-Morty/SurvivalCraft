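; Item container component that stores inventory items in a slot array on its owner.
; A server-named event calls AddItem, which writes the item into the first slot with an ItemID of zero and reports failure when none is free.
; UpdateUI forwards the changed slot to the owning character's controller through message calls, handling only the Player Inventory container type and no slot resets.
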(event Custom|AddItemOnServer
  (params (Item :type S%20Item%20Info%20Structure))
  (CallFunction|AddItem Item))

(fn FindEmptySlot
  (bind (_array_element _array_index) (Utilities|Array|ForEachLoopwithBreak (Variables|Default|GetItems) :!label _label)
    (:LoopBody
      (if (== (.ItemID (Utilities|Struct|BreakS_ItemInfo _array_element)) 0)
        (LocalVariables|SetEmptySlotIndex _array_index)
        (LocalVariables|SetFoundEmptySlot? true)
        (goto _label Break)))
    (:Completed
      (return (LocalVariables|GetFoundEmptySlot?) (LocalVariables|GetEmptySlotIndex)))))

(fn AddItem
  (params (Item :type S%20Item%20Info%20Structure))
  (LocalVariables|SetLocalItemInfo Item)
  (bind (_success_ _emptyindex) (CallFunction|FindEmptySlot))
  (if _success_
    (bind _output_get (LocalVariables|SetLocalEmptyIndex _emptyindex))
    (Utilities|Array|SetArrayElem (Variables|Default|GetItems) _output_get (LocalVariables|GetLocalItemInfo))
    (CallFunction|UpdateUI (LocalVariables|GetLocalEmptyIndex) (LocalVariables|GetLocalItemInfo) false)
    (return true)
    (else
      (return false))))

(fn UpdateUI
  (params (Index :type Integer) (ItemInfo :type S%20Item%20Info%20Structure) (ResetSlot? :type Boolean))
  (if (not ResetSlot?)
    (switch Utilities|FlowControl|Switch|SwitchonE_ContainerType (Variables|Default|GetContainerType)
      (:NewEnumerator0
        (bind _controllerref (Class|BPISurvivalCraft|GetControllerfromChar(Message) (Components|GetOwner)))
        (Default|UpdateItemSlot _controllerref "NewEnumerator0" Index ItemInfo)))))