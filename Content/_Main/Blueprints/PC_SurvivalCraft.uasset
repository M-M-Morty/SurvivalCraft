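; Player controller for a survival crafting game that owns the main HUD widget and handles the inventory UI.
; On BeginPlay it creates W_MainWidget only on the Remote authority branch.
; Tab or I toggles inventory visibility, switching input mode and mouse cursor along with it.
; UpdateItemSlot pushes item info into the inventory grid slot at the given index, ignoring its Container input.
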(event Custom|InventoryOnClient
  (if (Variables|Default|GetInventoryShown?)
    (Default|SetinventoryVis (Variables|Default|GetMainWidgetRef) false)
    (Input|SetInputModeGameOnly self false)
    (Variables|Default|SetbShowMouseCursor false)
    (Variables|Default|SetInventoryShown? false)
    (else
      (Default|SetinventoryVis (Variables|Default|GetMainWidgetRef) true)
      (Input|SetInputModeGameandUI self 0 "DoNotLock" true false)
      (Variables|Default|SetbShowMouseCursor true)
      (Variables|Default|SetInventoryShown? true))))

(event Custom|UpdateItemSlot
  (params (Container :type E_ContainerType%20Enum :default "NewEnumerator0") (Index :type Integer) (ItemInfo :type S%20Item%20Info%20Structure))
  (bind _mainwidgetref (Variables|Default|GetMainWidgetRef))
  (bind _w_inventory (Variables|/Game/_Main/Widgets/InventoryWidgets/W_MainWidget.W_MainWidget_C|GetW_Inventory _mainwidgetref))
  (bind _w_itemcontainergrid (Variables|/Game/_Main/Widgets/InventoryWidgets/W_Inventory.W_Inventory_C|GetW_ItemContainerGrid _w_inventory))
  (bind _slots (Variables|/Game/_Main/Widgets/InventoryWidgets/W_ItemContainerGrid.W_ItemContainerGrid_C|GetSlots _w_itemcontainergrid))
  (bind _output (Utilities|Array|Get(acopy) _slots Index))
  (Utilities|IsValid _output
    (:Is%20Valid
      (Default|UpdateSlot _output ItemInfo))))

(event EventBeginPlay
  (Networking|SwitchHasAuthority
    (:Remote
      (bind _returnvalue (UserInterface|CreateWidget "/Game/_Main/Widgets/InventoryWidgets/W_MainWidget.W_MainWidget_C" self))
      (bind _output_get (Variables|Default|SetMainWidgetRef _returnvalue))
      (UserInterface|Viewport|AddtoViewport _output_get 0))))

(event Input|KeyboardEvents|Tab
  (params (Key :type Key%20Structure :default "None"))
  (:Pressed
    (CallFunction|InventoryonClient)))

(event Input|KeyboardEvents|I
  (params (Key :type Key%20Structure :default "None"))
  (:Pressed
    (CallFunction|InventoryonClient)))

(fn ConstructionScript)

(fn PlayerControllerRef
  (return self))